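; Game instance for the NetShoot multiplayer shooter that manages online sessions and starts the match.
; Hosting creates a session and opens the room map as a listen server; searches feed the main menu list and joining shows a loading screen.
; Exits and pending-connection failures destroy the session, so rejected joins don't block later ones.
; On match start, the server swaps streamed levels, then spawns and possesses characters at PlayerStarts by index.
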(event Custom|HostGameRoom
  (|Session (Game|GetPlayerController 0) (Variables|Default|GetPublic%20Connections) (Variables|Default|GetUseLan)
    (:OnSuccess
      (Development|PrintString "Hello")
      ;[1 1 1] 打开新的关卡后开始监听，注意如果再次打开别的关卡，则会自动断开链接（与SetClientTravel有关
      (Game|OpenLevel(byName) "SessionRoomLevel" true "listen") ; 最重要的就是这个，Options中添加listen\n它可以使得一个Standalone或者Client变成一个Server
    )
    (:OnFailure
      (Development|PrintString "CreateSession Error"))))

(event Custom|SearchRoom
  (bind _results (|FindSessions (Game|GetPlayerController 0) 100 (Variables|Default|GetUseLan))
    (:then
      (Development|PrintString "SearchingSession"))
    (:OnSuccess
      (for _array_element _results
        (Default|AddSessionItem (Variables|Default|GetMainMenuWidget) _array_element))
      (Default|CloseLoading (Variables|Default|GetMainMenuWidget) :!label _label))
    (:OnFailure
      (Development|PrintString "SearchSession Error")
      (goto _label))))

(event Custom|JoinRoom
  (params (Session :type Blueprint%20Session%20Result%20Structure))
  (|JoinSession (Game|GetPlayerController 0) Session
    (:then
      (Viewport|RemoveAllWidgets)
      (bind _returnvalue (UserInterface|CreateWidget "/Game/AUI/MenuUI/LoadingOverall.LoadingOverall_C"))
      (UserInterface|Viewport|AddtoViewport _returnvalue 0))
    (:OnSuccess
      (Development|PrintString "JoinSession"))
    (:OnFailure
      (Development|PrintString "JoinSession Error"))))

(event Custom|HostStartGame
  (Utilities|FlowControl|Sequence
    (:then_0
      ;[1 1 1] only server run this
      (if (Networking|IsServer)
        (Game|LoadStreamLevel(byName) "GameMap" true)
        (Game|UnloadStreamLevel(byName) "SessionRoomUILevel" false)
        (bind _asnet_shoot_game_game_mode (Utilities|Casting|CastToNetShootGameGameMode (Game|GetGameMode)))
        (Class|NetShootGameGameMode|StartGame _asnet_shoot_game_game_mode)
        (for _index (range 0 5)
          (Utilities|IsValid (Game|GetPlayerController _index)
            (:Is%20Valid
              (bind _returnvalue (Utilities|SpawnCharacteratPlayerStart _index))
              (Pawn|Possess (Game|GetPlayerController _index) _returnvalue)
              (bind _asbp_net_shoot_player_controller (Utilities|Casting|CastToBP_NetShootPlayerController (Game|GetPlayerController _index)))
              (Default|ActiveUI _asbp_net_shoot_player_controller))))))))

(event Custom|ExitRoom
  (|DestroySession (Game|GetPlayerController 0)
    (:OnSuccess
      _)
    (:OnFailure
      (Development|PrintString "Back to menu false to destroy session")))
  (Game|OpenLevel(byName) "MainMenuLevel") ; 只有打开新地图才能彻底关闭会话
  (Development|PrintString "Bye"))

(event EventHandleNetworkError
  (params (FailureType :type ENetworkFailure%20Enum :default "NetDriverAlreadyExists") (bIsServer :type Boolean))
  ;[1 1 1] 用于解决JoinGame后被PreLogin拒绝，没有断开会话，进而导致不能再创建或进入其他会话的问题
  (Development|PrintString (Utilities|String|EnumtoString FailureType))
  (switch Utilities|FlowControl|Switch|SwitchonENetworkFailure FailureType
    (:PendingConnectionFailure
      (|DestroySession (Game|GetPlayerController 0)
        (:OnSuccess
          (Development|PrintString "Destroy Session"))))))