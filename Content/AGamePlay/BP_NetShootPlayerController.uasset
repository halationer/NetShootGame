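; Player controller for a networked shooter that manages the local player's main game UI.
; ReActiveUI replaces only the MainGameUI widget, while ActiveUI clears all widgets before creating it, which the author notes disables movement on mobile.
; Both act only on the local controller and cache the nested PlayerStateUI.
; ShowPlayerState toggles that panel, collapsing it or restoring it through its ReVisUI call.
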(event Custom|ActiveUI
  (if (Pawn|IsLocalPlayerController)
    (Viewport|RemoveAllWidgets)
    (bind _returnvalue (UserInterface|CreateWidget "/Game/AUI/InGameUI/MainGameUI.MainGameUI_C" 0 0))
    (bind _output_get (Variables|Default|SetMainGameUI _returnvalue))
    (UserInterface|Viewport|AddtoViewport _output_get 0)
    (Variables|Default|SetPlayerStateUI (Variables|/Game/AUI/InGameUI/MainGameUI.MainGameUI_C|GetPlayerStateUI _output_get))))

(event Custom|ReActiveUI
  (if (Pawn|IsLocalPlayerController)
    (Utilities|IsValid (Variables|Default|GetMainGameUI)
      (:Is%20Valid
        (Widget|RemovefromParent (Variables|Default|GetMainGameUI)))
      (:Is%20Not%20Valid
        _))
    (bind _returnvalue (UserInterface|CreateWidget "/Game/AUI/InGameUI/MainGameUI.MainGameUI_C" 0 0))
    (bind _output_get (Variables|Default|SetMainGameUI _returnvalue))
    (UserInterface|Viewport|AddtoViewport _output_get 0)
    (Variables|Default|SetPlayerStateUI (Variables|/Game/AUI/InGameUI/MainGameUI.MainGameUI_C|GetPlayerStateUI _output_get))))

(event EventShowPlayerState
  (bind _playerstateui (Variables|Default|GetPlayerStateUI))
  (switch Utilities|FlowControl|Switch|SwitchonESlateVisibility (Widget|GetVisibility _playerstateui)
    (:Visible
      (Widget|SetVisibility _playerstateui "Collapsed"))
    (:Collapsed
      (Default|ReVisUI _playerstateui))))

(fn ConstructionScript)