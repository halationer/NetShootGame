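; BP_WeaponBaseComponent is a skeletal mesh weapon component that shows a weapon and fires physical projectiles.
; A server-named event sets the WeaponAttribute struct, whose RepNotify swaps in the matching skeletal mesh.
; Fire spawns a BulletBase at the Muzzle socket, oriented to the player controller's control rotation, and launches it with a physics impulse.
; It also draws a debug line along the aim direction.
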(event Custom|OnRep_WeaponAttribute
  ;[1 1 1] WeaponAttribute Sync
  (Class|SkinnedMeshComponent|SetSkeletalMesh (.SkeletonMesh (Utilities|Struct|BreakWeaponAttribute (Variables|Default|GetWeaponAttribute))) true))

(event Custom|Fire
  (params (Controller :type Controller%20Object%20Reference))
  (bind _returnvalue (Transformation|GetSocketLocation "Muzzle"))
  (bind _as玩家控制器 (Utilities|Casting|CastToPlayerController Controller))
  (Rendering|Debug|DrawDebugLine _returnvalue (+ (* (Math|Rotator|GetRotationXVector (Pawn|GetControlRotation _as玩家控制器 :!class /Script/Engine.Controller)) 1e+03) _returnvalue) "(R=1.000000,G=0.000000,B=0.000000,A=1.000000)" 5.0 0.0)
  (bind _returnvalue_2 (Game|SpawnActorfromClass "/Game/AWeapons/BulletBase.BulletBase_C" (Math|Transform|MakeTransform _returnvalue (Pawn|GetControlRotation _as玩家控制器 :!class /Script/Engine.Controller)) "Undefined" 0 0))
  (Physics|AddImpulse (Variables|/Game/AWeapons/BulletBase.BulletBase_C|GetBulletMesh _returnvalue_2) (* (Math|Rotator|GetRotationXVector (Pawn|GetControlRotation _as玩家控制器 :!class /Script/Engine.Controller)) 1e+04) "None" false))

(event Custom|SetWeaponAttributeServer
  (params (WeaponAttribute :type Weapon%20Attribute%20Structure))
  ;[1 1 1] WeaponAttribute Sync
  (Variables|Default|SetWeaponAttribute WeaponAttribute))