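; BP_WeaponActor is a weapon actor that gives itself a random weapon type from the WeaponList data table.
; RandomInit, called by the level script, picks a random row on the authority and applies it to WeaponMesh through SetWeaponAttribute.
; A SpotLightTest graph holds disconnected muzzle-light logic (intensity timeline, looping fire timer) that never runs, with empty BeginPlay and Fire events.
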(event Custom|RandomInit
  ;[1 1 1] Random init weapon type, according to the data table
  (Networking|SwitchHasAuthority
    (:Authority
      (bind _outrownames (DataTable|GetDataTableRowNames "/Game/Configs/WeaponList.WeaponList"))
      (bind _returnvalue (Utilities|GetDataTableRow "/Game/Configs/WeaponList.WeaponList" (.OutItem (Utilities|Array|Random _outrownames)))
        (:then
          (Class|WeaponBaseComponent|SetWeaponAttribute (Variables|Default|GetWeaponMesh) _returnvalue))))))

(fn ConstructionScript)

(event Custom|Fire)

(event EventBeginPlay)